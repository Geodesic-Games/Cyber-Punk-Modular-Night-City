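; Billboard actor that cycles its screen through random materials during play, with the mesh set at construction.
; On BeginPlay, if the material array has entries, it starts the LoopingPlay timeline.
; Each time the timeline finishes, it applies a random material to the configured slot and restarts.
; An unused SetMedia function would open a video media source through a dynamic material's "Video" texture parameter.
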(event `self.ReceiveBeginPlay`
  (if (not (`KismetArrayLibrary.Array_IsEmpty` (`self.BillboardMaterial`)))
    (`Timeline|LoopingPlay` :`NewTime` (`KismetMathLibrary.Conv_IntToDouble` (`self.Delay`)) :!via `PlayFromStart` :!label _label
      (:`Finished`
        (`PrimitiveComponent.SetMaterial` (`self.StaticMesh`) (`self.MaterialBillboard Index Element`) (`|GetArrayItem` (`self.BillboardMaterial`) (`KismetMathLibrary.RandomIntegerInRange` 0 (- (`KismetArrayLibrary.Array_Length` (`self.BillboardMaterial`)) 1))))
        (goto _label :!via `PlayFromStart`)))))

(fn `SetMedia`
  (bind _materialbillboard_index_element (`self.MaterialBillboard Index Element`))
  (bind _returnvalue (`PrimitiveComponent.CreateDynamicMaterialInstance` (`self.StaticMesh`) _materialbillboard_index_element (`PrimitiveComponent.GetMaterial` (`self.StaticMesh`) _materialbillboard_index_element) "None"))
  (bind _returnvalue_2 (`MaterialInstanceDynamic.K2_GetTextureParameterValue` _returnvalue "Video"))
  (`/Engine/EditorBlueprintResources/StandardMacros.IsValid` _returnvalue_2
    (:`Is Valid`
      (`PrimitiveComponent.SetMaterial` (`self.StaticMesh`) _materialbillboard_index_element _returnvalue)
      (bind _asmedia_texture (cast `MediaTexture` _returnvalue_2)
        (:`then`
          (bind _returnvalue_3 (`MediaPlayer.OpenSource` (`MediaTexture.GetMediaPlayer` _asmedia_texture) null))
          (if (not _returnvalue_3)
            (`KismetSystemLibrary.PrintString` "Failed to Open Media Source")))
        (:`CastFailed`
          (`KismetSystemLibrary.PrintString` "Failed to find MediaTexture"))))
    (:`Is Not Valid`
      (`KismetSystemLibrary.PrintString` "Video parameter is not valid."))))

(fn `UserConstructionScript`
  (`StaticMeshComponent.SetStaticMesh` (`self.StaticMesh`) (`self.New Mesh`)))